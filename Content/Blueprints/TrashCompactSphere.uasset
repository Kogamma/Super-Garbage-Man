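; Trash compactor kill volume that "kills" characters entering its sphere by stopping them and teleporting them to a random PlayerStart, cached on BeginPlay.
; A character carrying garbage loses the bag, decrementing the game instance's bags-left count and resetting pickup and animation state.
; An empty-handed character takes a score penalty through the game mode.
; Each death plays a random scream in 2D with varied pitch.
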(event OnComponentBeginOverlap(Sphere1)
  (params (OverlappedComponent :type Primitive%20Component%20Object%20Reference) (OtherActor :type Actor%20Object%20Reference) (OtherComp :type Primitive%20Component%20Object%20Reference) (OtherBodyIndex :type Integer) (bFromSweep :type Boolean) (SweepResult :type Hit%20Result%20Structure%20%28by%20ref%29))
  (bind _spawn_points (Variables|Default|GetSpawn%20Points))
  ;[1 1 1] Respawns the character at a random player start and removes the trashbag from their hand and from the game.
  (Utilities|FlowControl|Sequence
    (:then_0
      (bind _asue_4asp_character (Utilities|Casting|CastToUe4ASP_Character OtherActor))
      (Variables|/Script/Engine.MovementComponent|SetVelocity (Variables|/Script/Engine.Character|GetCharacterMovement _asue_4asp_character) "0, 0, 0")
      (Transformation|SetActorTransform _asue_4asp_character (Utilities|Array|Get(acopy) _spawn_points (Math|Random|RandomInteger (Utilities|Array|Length _spawn_points))))
      (bind _asue_4asp_character_2 (Utilities|Casting|CastToUe4ASP_Character OtherActor))
      (if (Variables|/Game/AnimStarterPack/Animations/Ue4ASP_Character.Ue4ASP_Character_C|GetHasGarbage _asue_4asp_character_2)
        (Default|Dequipped _asue_4asp_character_2)
        (bind _asmy_game_instance (Utilities|Casting|CastTomyGameInstance (Game|GetGameInstance)))
        (Default|DecrementTrashbagsLeft _asmy_game_instance)
        (Variables|/Game/AnimStarterPack/Animations/Ue4ASP_Character.Ue4ASP_Character_C|SetCanPickUp _asue_4asp_character_2 true)
        (bind _output_get (Variables|/Game/AnimStarterPack/Animations/Ue4ASP_Character.Ue4ASP_Character_C|SetHasGarbage _asue_4asp_character_2 false))
        (bind _asue4asp_hero_tpp_anim_blueprint (Utilities|Casting|CastToUE4ASP_HeroTPP_AnimBlueprint (Components|SkeletalMesh|GetAnimInstance (Variables|/Script/Engine.Character|GetMesh _asue_4asp_character_2))))
        (Variables|/Game/AnimStarterPack/Animations/UE4ASP_HeroTPP_AnimBlueprint.UE4ASP_HeroTPP_AnimBlueprint_C|SetHolding%20Garbage _asue4asp_hero_tpp_anim_blueprint _output_get)
        (else
          (bind _asgame_bp (Utilities|Casting|CastToGame_BP (Game|GetGameMode)))
          (Default|UpdateScore _asgame_bp _asue_4asp_character_2 -10))))
    (:then_2
      ;[1 1 1] Plays a randomly picked screaming sound when the player 'dies'
      (Audio|PlaySound2D (Utilities|Array|Get(acopy) (Variables|Default|GetSounds) (Math|Random|RandomIntegerinRange 0 2)) 0.1 (Math|Random|RandomFloatinRange 0.8 1.0)))))

(event EventBeginPlay
  (bind _sounds (Variables|Default|GetSounds))
  ;[1 1 1] Finds all the player start objects in the level
  (Utilities|FlowControl|Sequence
    (:then_0
      (bind _outactors (Actor|GetAllActorsOfClass "/Script/Engine.PlayerStart"))
      (for (_array_element _array_index) _outactors
        (Utilities|Array|SetArrayElem (Variables|Default|GetSpawn%20Points) _array_index (Transformation|GetActorTransform _array_element) true)))
    (:then_1
      ;[1 1 1] Adds all the screaming sounds to an array so we can randomly pick one of them later
      (Utilities|Array|Add _sounds "/Game/SFX/Screams/Scream_2_Cue.Scream_2_Cue")
      (Utilities|Array|Add _sounds "/Game/SFX/Screams/Scream_5_Cue.Scream_5_Cue")
      (Utilities|Array|Add _sounds "/Game/SFX/Screams/Scream_7_Cue.Scream_7_Cue"))))

(fn ConstructionScript)