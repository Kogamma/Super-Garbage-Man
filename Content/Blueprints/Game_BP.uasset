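; Game_BP sets up local multiplayer matches and ends them when no trash bags remain.
; On BeginPlay outside the menu and results levels, it stores the PickUpTrash count in myGameInstance, creates extra local players from PlayerAmount, and starts one of three random music cues.
; Tick polls the game instance's remaining bag count outside the results level; at zero it stops the music, switches to UI-only input and opens lvl_MatchResults.
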(event EventBeginPlay
  ;[1 1 1] PlayerCreation
  (Utilities|FlowControl|Sequence
    (:then_0
      (bind _returnvalue (Game|GetCurrentLevelName true))
      (if (and (Utilities|Enum|NotEqual(Enum) "MainMenu" _returnvalue) (Utilities|Enum|NotEqual(Enum) _returnvalue "lvl_MatchResults"))
        (bind _asmy_game_instance (Utilities|Casting|CastTomyGameInstance (Game|GetGameInstance)))
        (bind _outactors (Actor|GetAllActorsOfClass "/Game/Blueprint_Assets/pickUpTrash.pickUpTrash_C"))
        (Variables|/Game/Blueprints/myGameInstance.myGameInstance_C|SetNrTrashbagsLeft _asmy_game_instance (Utilities|Array|Length _outactors))
        (bind _asmy_game_instance_2 (Utilities|Casting|CastTomyGameInstance (Game|GetGameInstance)))
        (bind _output_get (Variables|Default|SetPlayerAmount (Variables|/Game/Blueprints/myGameInstance.myGameInstance_C|GetPlayerAmount _asmy_game_instance_2)))
        (Class|GameplayStatics|CreatePlayer -1)
        (if (>= _output_get 3)
          (Class|GameplayStatics|CreatePlayer -1)
          (if (>= _output_get 4)
            (Class|GameplayStatics|CreatePlayer -1)))))
    (:then_1
      ;[1 1 1] If the level that started was not a menu level the game randomizes one of the three music cues and then loops that for the rest of the match
      (bind _returnvalue_2 (Game|GetCurrentLevelName true))
      (if (and (Utilities|Enum|NotEqual(Enum) "MainMenu" _returnvalue_2) (Utilities|Enum|NotEqual(Enum) "lvl_MatchResults" _returnvalue_2))
        (bind _output_get_2 (Variables|Default|SetMusicIndex (Math|Random|RandomIntegerinRange 0 2)))
        (Utilities|FlowControl|Sequence
          (:then_0
            (if (== 0 _output_get_2)
              (bind _returnvalue_3 (AddComponent|AddAudioComponent false))
              (Audio|Components|Audio|Play _returnvalue_3 0.0)
              (Variables|Default|SetCurrentCue _returnvalue_3)))
          (:then_1
            (if (== 1 _output_get_2)
              (bind _returnvalue_4 (AddComponent|AddAudioComponent false))
              (Audio|Components|Audio|Play _returnvalue_4 0.0)
              (Variables|Default|SetCurrentCue _returnvalue_4)))
          (:then_2
            (if (== _output_get_2 2)
              (bind _returnvalue_5 (AddComponent|AddAudioComponent false))
              (Audio|Components|Audio|Play _returnvalue_5 0.0)
              (Variables|Default|SetCurrentCue _returnvalue_5))))))))

(event EventTick
  (params (DeltaSeconds :type Float%20%28single-precision%29))
  ;[1 1 1] Ends the match and goes to the results level if all the trashbags are gone. Also stops the music
  (bind _returnvalue (Game|GetCurrentLevelName true))
  (if (Utilities|Enum|NotEqual(Enum) _returnvalue "lvl_MatchResults")
    (bind _asmy_game_instance (Utilities|Casting|CastTomyGameInstance (Game|GetGameInstance)))
    (bind _nrtrashbagsleft (Default|NrOfTrashbagsLeft _asmy_game_instance))
    (if (<= _nrtrashbagsleft 0)
      (Audio|Components|Audio|Stop (Variables|Default|GetCurrentCue))
      (Input|SetInputModeUIOnly (Game|GetPlayerController 0) 0 "DoNotLock")
      (Game|OpenLevel(byName) "lvl_MatchResults"))))

(fn ConstructionScript)