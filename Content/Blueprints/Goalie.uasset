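; Goalie character that patrols side to side along the Y axis and blocks thrown trashbags.
; Tick feeds movement input along a direction that flips when the Y position passes the min or max bound.
; Overlapping a pickUpTrash decrements the trashbags-left count in the game instance, destroys the bag and briefly flashes the mesh's BodyColor material parameter red.
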(event Collision|EventActorBeginOverlap
  (params (OtherActor :type Actor%20Object%20Reference))
  ;[1 1 1] If the goalie gets hit by a trashbag, the trashbag gets destroyed
  (bind _aspick_up_trash (Utilities|Casting|CastTopickUpTrash OtherActor))
  (bind _asmy_game_instance (Utilities|Casting|CastTomyGameInstance (Game|GetGameInstance)))
  (Default|DecrementTrashbagsLeft _asmy_game_instance)
  (Actor|DestroyActor _aspick_up_trash)
  (Rendering|Material|SetVectorParameterValueonMaterials (Variables|Character|GetMesh) "BodyColor" (+ "0.450000,0.406000,0.362000" "0.550000,-0.300000,-0.260000"))
  (Utilities|FlowControl|Delay 0.2)
  (Rendering|Material|SetVectorParameterValueonMaterials (Variables|Character|GetMesh) "BodyColor" (+ "0.450000,0.406000,0.362000" "0.000000, 0, 0")))

(event EventTick
  (params (DeltaSeconds :type Float%20%28single-precision%29))
  (bind _returnvalue (Transformation|GetActorLocation))
  (bind _y (Math|Vector|BreakVector _returnvalue))
  ;[1 1 1] Makes the goalie move back and forth between two set min and max points
  (Pawn|Input|AddMovementInput (Variables|Default|GetDirection) (Variables|Default|GetGoalieSpeed) false)
  (Utilities|FlowControl|Sequence
    (:then_0
      (if (> _y (Variables|Default|GetMaxPos))
        (bind _output_get (Variables|Default|SetDirection "0.000000,-1.000000,0.000000"))
        (Variables|Default|SetDirection _output_get)))
    (:then_1
      (if (< _y (Variables|Default|GetMinPos))
        (bind _output_get_2 (Variables|Default|SetDirection "0,1.000000, 0"))
        (Variables|Default|SetDirection _output_get_2)))))

(fn ConstructionScript)