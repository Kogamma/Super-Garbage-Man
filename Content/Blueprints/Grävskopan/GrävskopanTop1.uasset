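; Drivable excavator character with a wrecking ball that launches characters it hits, making them drop their bag and briefly delaying pickup re-enabling.
; A character holding the steering wheel who hits its mesh is hidden while their controller possesses the excavator, which uses axis-driven movement and rotation.
; After a timed ride, control returns, the excavator resets, the player moves to a random cached PlayerStart, and a missing steering wheel respawns after a delay.
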(event OnComponentHit(WreckingBall)
  (params (HitComponent :type Primitive%20Component%20Object%20Reference) (OtherActor :type Actor%20Object%20Reference) (OtherComp :type Primitive%20Component%20Object%20Reference) (NormalImpulse :type Vector :default "0, 0, 0") (Hit :type Hit%20Result%20Structure%20%28by%20ref%29))
  ;[1 1 1] Launch characters that come in contact with the wreckingball!
  (bind _asue_4asp_character (Utilities|Casting|CastToUe4ASP_Character OtherActor))
  (Character|LaunchCharacter _asue_4asp_character (+ (* (Math|Vector|GetForwardVector (Transformation|GetActorRotation)) 300) "0, 0,400.000000") false false)
  (Audio|PlaySound2D "/Game/SFX/WreckingBall_Cue.WreckingBall_Cue" 1.0 (Math|Random|RandomFloatinRange 0.5 1.0))
  (Default|DropBag _asue_4asp_character)
  (Utilities|FlowControl|Delay 0.4)
  (Utilities|IsValid 0
    (:Is%20Valid
      (Variables|/Game/AnimStarterPack/Animations/Ue4ASP_Character.Ue4ASP_Character_C|SetCanPickUp _asue_4asp_character true))))

(event OnComponentHit(StaticMesh7)
  (params (HitComponent :type Primitive%20Component%20Object%20Reference) (OtherActor :type Actor%20Object%20Reference) (OtherComp :type Primitive%20Component%20Object%20Reference) (NormalImpulse :type Vector :default "0, 0, 0") (Hit :type Hit%20Result%20Structure%20%28by%20ref%29))
  ;[1 1 1] Possess the Wreckingball!
  (bind _asue_4asp_character (Utilities|Casting|CastToUe4ASP_Character OtherActor))
  (if (Variables|/Game/AnimStarterPack/Animations/Ue4ASP_Character.Ue4ASP_Character_C|GetHasSteeringWheel _asue_4asp_character)
    (Pawn|Possess (Pawn|GetController _asue_4asp_character) self)
    (Transformation|SetActorLocation _asue_4asp_character (Variables|Default|GetHiddenSpot) false false)
    (Utilities|FlowControl|Delay 25.0)
    (Pawn|Possess (Pawn|GetController) _asue_4asp_character)
    (Transformation|SetActorLocation "11.000000,0.000000,124.000000" false false)
    (Transformation|SetActorLocation _asue_4asp_character (Utilities|Array|Get(acopy) (Variables|Default|GetSpawnpoints) (Math|Random|RandomIntegerinRange 0 3)) false false)
    (Variables|/Game/AnimStarterPack/Animations/Ue4ASP_Character.Ue4ASP_Character_C|SetHasSteeringWheel _asue_4asp_character false)
    ;[1 1 1] Respawns the steering wheel!
    (bind _outactors (Actor|GetAllActorsOfClass "/Game/Blueprint_Assets/TheSteeringWheel.TheSteeringWheel_C"))
    (if (not (> (Utilities|Array|Length _outactors) 0))
      (Utilities|FlowControl|Delay 1e+01)
      (Game|SpawnActorfromClass "/Game/Blueprint_Assets/TheSteeringWheel.TheSteeringWheel_C" (Math|Transform|MakeTransform "856.000000,0.000000,306.000000" "0, 0, 0" "1.000000,1,1") "Undefined" 0 0))))

(event EventBeginPlay
  (bind _charactermovement (Variables|Character|GetCharacterMovement))
  ;[1 1 1] Character variables setup
  (Variables|/Script/Engine.CharacterMovementComponent|SetMaxWalkSpeed _charactermovement 8e+02)
  (Variables|/Script/Engine.CharacterMovementComponent|SetGroundFriction _charactermovement 3.0)
  (bind _outactors (Actor|GetAllActorsOfClass "/Script/Engine.PlayerStart"))
  (for _array_element _outactors
    (Utilities|Array|Add (Variables|Default|GetSpawnpoints) (Transformation|GetActorLocation _array_element))))

(event Input|AxisEvents|InputAxisMoveUp
  (params (AxisValue :type Float%20%28single-precision%29))
  ;[1 1 1] Movement
  (Pawn|Input|AddMovementInput "1.000000, 0, 0" AxisValue false))

(event Input|AxisEvents|InputAxisMoveRight
  (params (AxisValue :type Float%20%28single-precision%29))
  ;[1 1 1] Movement
  (Pawn|Input|AddMovementInput "0,1.000000, 0" AxisValue false))

(event Input|AxisEvents|InputAxisLookUp
  (params (AxisValue :type Float%20%28single-precision%29))
  ;[1 1 1] Rotation
  (if (> (Math|Vector|VectorLength (Math|Vector|MakeVector AxisValue (stale Input|AxisEvents|InputAxisLookRight AxisValue) 0.0)) 0.25)
    (Pawn|SetControlRotation (Pawn|GetController) (Math|Interpolation|RInterpTo (Transformation|GetActorRotation self) (Math|Conversions|RotationFromXVector (Math|Vector|MakeVector AxisValue (stale Input|AxisEvents|InputAxisLookRight AxisValue) 0.0)) 0.5 0.05))))

(event Input|AxisEvents|InputAxisLookRight
  (params (AxisValue :type Float%20%28single-precision%29))
  ;[1 1 1] Rotation
  (if (> (Math|Vector|VectorLength (Math|Vector|MakeVector (stale Input|AxisEvents|InputAxisLookUp AxisValue) AxisValue 0.0)) 0.25)
    (Pawn|SetControlRotation (Pawn|GetController) (Math|Interpolation|RInterpTo (Transformation|GetActorRotation self) (Math|Conversions|RotationFromXVector (Math|Vector|MakeVector (stale Input|AxisEvents|InputAxisLookUp AxisValue) AxisValue 0.0)) 0.5 0.05))))

(fn ConstructionScript)