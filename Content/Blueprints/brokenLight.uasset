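; Broken light Blueprint that makes its SpotLight flicker by repeatedly toggling visibility.
; Tick passes through a DoOnce into a Retriggerable Delay, then toggles the light and resets the gate for the next cycle.
; The delay's random range is zero at both ends, so flicker is rapid rather than randomly timed.
; An unconnected chain with randomized delays and paired toggles never runs.
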(event EventTick
  (params (DeltaSeconds :type Float%20%28single-precision%29))
  (Utilities|FlowControl|DoOnce false :!label _label
    (:Completed
      (Utilities|FlowControl|RetriggerableDelay (Math|Random|RandomFloatinRange 0.0 0.0))
      (Rendering|ToggleVisibility (Variables|Default|GetSpotLight) false)
      (goto _label Reset))))

(fn ConstructionScript)