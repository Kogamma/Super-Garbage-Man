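; TC_SL is a level actor that respawns the player when a Garbage_Man_Blueprint character overlaps it.
; On overlap, it moves player character 0 to the stored SpawnPoint transform, then calls Dequipped on the overlapping garbage man if it has garbage.
; A PlayerReSpawn function exposes SpawnPoint, though the overlap event reads the variable directly.
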(event Collision|EventActorBeginOverlap
  (params (OtherActor :type Actor%20Object%20Reference))
  ;[1 1 1] Respawn Character
  (Utilities|Casting|CastToGarbage_Man_Blueprint OtherActor)
  (Transformation|SetActorTransform (Game|GetPlayerCharacter 0) (Variables|Default|GetSpawn%20Point))
  (bind _asgarbage_man_blueprint (Utilities|Casting|CastToGarbage_Man_Blueprint OtherActor))
  (bind _hasgarbage (Default|HasGarbage _asgarbage_man_blueprint))
  (if _hasgarbage
    (Default|Dequipped _asgarbage_man_blueprint)))

(fn ConstructionScript)

(fn PlayerReSpawn
  ;[1 1 1] Player ReSpawn
  (return (Variables|Default|GetSpawn%20Point)))