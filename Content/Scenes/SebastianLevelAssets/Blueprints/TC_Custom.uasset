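; TC_Custom is an overlap-triggered respawn actor that sends the Garbage Man character back to a spawn point.
; On overlap it casts to Garbage_Man_Blueprint and sets that character's transform to SpawnPoint, without sweeping.
; If the character has garbage, it calls Dequipped and decrements the trashbags-left count in myGameInstance.
; A PlayerReSpawn function exposes SpawnPoint, and the construction script is empty.
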(event Collision|EventActorBeginOverlap
  (params (OtherActor :type Actor%20Object%20Reference))
  ;[1 1 1] Respawn Character
  (bind _asgarbage_man_blueprint (Utilities|Casting|CastToGarbage_Man_Blueprint OtherActor))
  (Transformation|SetActorTransform _asgarbage_man_blueprint (Variables|Default|GetSpawn%20Point))
  (bind _asgarbage_man_blueprint_2 (Utilities|Casting|CastToGarbage_Man_Blueprint OtherActor))
  (bind _hasgarbage (Default|HasGarbage _asgarbage_man_blueprint_2))
  (if _hasgarbage
    (Default|Dequipped _asgarbage_man_blueprint_2)
    (bind _asmy_game_instance (Utilities|Casting|CastTomyGameInstance (Game|GetGameInstance)))
    (Default|DecrementTrashbagsLeft _asmy_game_instance)))

(fn ConstructionScript)

(fn PlayerReSpawn
  ;[1 1 1] Player ReSpawn
  (return (Variables|Default|GetSpawn%20Point)))