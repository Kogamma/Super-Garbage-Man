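; Sewage static mesh Blueprint that animates the actor with continuous rotation and a timeline-driven elevation offset.
; Tick re-applies the current rotation, then adds SewageRotationRate as a local rotation each frame, without delta-time scaling.
; BeginPlay stores the start location and plays a timeline whose track is added to it to set the actor's position.
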(event EventTick
  (params (DeltaSeconds :type Float%20%28single-precision%29))
  ;[1 1 1] Rotation Mechanic
  (bind _output_get (Variables|Default|SetSewageStartRotPos (Transformation|GetActorRotation self)))
  (Transformation|SetActorRotation self _output_get)
  (Transformation|AddActorLocalRotation (Variables|Default|GetSewageRotationRate) false false))

(event EventBeginPlay
  ;[1 1 1] Elevation Mechanic
  (Variables|Default|SetStartLocation (Transformation|GetActorLocation self))
  (bind _newtrack_1 (Timeline|Timeline_0 Play)
    (:Update
      (Transformation|SetActorLocation self (+ _newtrack_1 (Variables|Default|GetStartLocation)) false false))))

(fn ConstructionScript)